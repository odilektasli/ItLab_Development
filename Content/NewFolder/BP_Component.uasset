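; BP_Component is a chainable component actor, apparently for a circuit simulation, with a voltage and a toggleable simulating state.
; The construction script gives the cube a dynamic material, which Tick colors green while simulating and red otherwise.
; A FlipFlop drives the state; only switching on cascades to a valid Next component.
; The cascade calls SetNextVoltage on Next, so Next copies its own Voltage onward, then toggles Next.
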(event Custom|ToggleSimulating
  (bind _next (Variables|Default|GetNext))
  (bind _isa (Utilities|FlowControl|FlipFlop)
    (:A
      _)
    (:B
      _))
  (bind _output_get (Variables|Default|SetIsSimulating _isa))
  (if _output_get
    (Utilities|IsValid _next
      (:Is%20Valid
        (CallFunction|SetNextVoltage _next)
        (CallFunction|ToggleSimulating _next)))))

(event Custom|SetNextVoltage
  (Variables|BP_Component_C|SetVoltage (Variables|Default|GetNext) (Variables|Default|GetVoltage)))

(event EventBeginPlay)

(event Collision|EventActorBeginOverlap
  (params (OtherActor :type Actor%20Object%20Reference)))

(event EventTick
  (params (DeltaSeconds :type Float%20%28single-precision%29))
  (bind _mymat (Variables|Default|GetMyMat))
  (if (Variables|Default|GetIsSimulating)
    (Rendering|Material|SetVectorParameterValue _mymat "Color" "(R=0.000000,G=1.000000,B=0.105791,A=1.000000)" :!class /Script/Engine.MaterialInstanceDynamic)
    (else
      (Rendering|Material|SetVectorParameterValue _mymat "Color" "(R=1.000000,G=0.000000,B=0.000000,A=1.000000)" :!class /Script/Engine.MaterialInstanceDynamic))))

(fn ConstructionScript
  (bind _returnvalue (Rendering|Material|CreateDynamicMaterialInstance (Variables|Default|GetCube) 0 "/Game/NewFolder/M_MyMAt.M_MyMAt" "None" :!class /Script/Engine.PrimitiveComponent))
  (Variables|Default|SetMyMat _returnvalue))